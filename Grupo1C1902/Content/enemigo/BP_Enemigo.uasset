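; BP_Enemigo is an enemy character that chases and attacks the player, driven by a state event, EstadosEnemigo, with animations per state.
; Idle polls every 0.2 seconds for a path and a nearby player, then Perseguir uses AIMoveTo, leading to Atack on success or Idle on failure.
; Damage requests RecibirDaño, which has no handler; the health and knockback logic is disconnected, and the ragdoll Muerte state is never requested.
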(event Custom|EstadosEnemigo
  (params (Estado :type Estados_Enemigo%20Enum :default "NewEnumerator0"))
  (switch Utilities|FlowControl|Switch|SwitchonEstados_Enemigo Estado
    (:NewEnumerator0
      (Components|Animation|PlayAnimation (Variables|Character|GetMesh) 0 true)
      (bind _returnvalue (Class|NavigationSystemV1|FindPathtoActorSynchronously (Transformation|GetActorLocation) (Game|GetPlayerCharacter 0) 5e+01 0 0 :!label _label))
      (if (not (Utilities|IsValid _returnvalue))
        (Utilities|FlowControl|Delay 0.2 :!label _label_2)
        (goto _label)
        (elif (< (Math|Vector|VectorLengthXY (- (Transformation|GetActorLocation) (Transformation|GetActorLocation (Game|GetPlayerCharacter 0)))) 5e+02)
          (CallFunction|EstadosEnemigo "NewEnumerator4")
          (else
            (goto _label_2)))))
    (:NewEnumerator1
      (Components|Animation|PlayAnimation (Variables|Character|GetMesh) 0 false)
      (Utilities|FlowControl|Delay 2.63)
      (CallFunction|EstadosEnemigo "NewEnumerator4"))
    (:NewEnumerator3
      (Physics|SetSimulatePhysics (Variables|Character|GetMesh) true))
    (:NewEnumerator4
      (Components|Animation|PlayAnimation (Variables|Character|GetMesh) 0 true)
      (AI|AIMoveTo self "0, 0, 0" (Game|GetPlayerCharacter 0) 5.0 false
        (:OnSuccess
          (CallFunction|EstadosEnemigo "NewEnumerator1"))
        (:OnFail
          (CallFunction|EstadosEnemigo "NewEnumerator0"))))))

(event EventBeginPlay
  (CallFunction|EstadosEnemigo "NewEnumerator0"))

(event Collision|EventActorBeginOverlap
  (params (OtherActor :type Actor%20Object%20Reference)))

(event EventTick
  (params (DeltaSeconds :type Float%20%28single-precision%29)))

(event Game|Damage|EventAnyDamage
  (params (Damage :type Float%20%28single-precision%29) (DamageType :type Damage%20Type%20Object%20Reference) (InstigatedBy :type Controller%20Object%20Reference) (DamageCauser :type Actor%20Object%20Reference))
  (CallFunction|EstadosEnemigo "NewEnumerator2"))

(fn ConstructionScript)